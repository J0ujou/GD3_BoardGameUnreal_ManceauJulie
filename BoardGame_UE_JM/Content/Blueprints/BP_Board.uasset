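; Board actor for a square-by-square board game, holding the ordered Case array of square actors and computing player moves along it.
; CalculateNewPosition adds a move count to the current index, bounces any overshoot back from the last square, clamps the result and reports the rebound.
; Helpers return the last index and a square's world location.
; BeginPlay prints a hard-coded test move and caches the last index.
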(event `self.ReceiveBeginPlay`
  ; test calcul de position
  (bind (_newposition _rebound) (`self.CalculateNewPosition` 15 3))
  (`KismetSystemLibrary.PrintString` (`KismetStringLibrary.Conv_IntToString` _newposition))
  (`KismetSystemLibrary.PrintString` (`KismetStringLibrary.Conv_BoolToString` _rebound))
  (bind _index (`self.GetlastIndex`))
  (set `self.LastBoardIndex` _index))

(fn `CalculateNewPosition`
  (params (Actual :type Integer) (Number :type Integer))
  (returns (NewPosition :type Integer) (Rebound :type Boolean))
  (bind _returnvalue (+ Actual Number))
  ; calcule la prochaine position du joueur
  (bind _index (`self.GetlastIndex`))
  (bind _output_get (set `self.TooMuch` (- _returnvalue _index)))
  (bind _output_get_2 (set `self.Rebound` (> _returnvalue _index)))
  (return (`KismetMathLibrary.Clamp` (`KismetMathLibrary.SelectInt` (- _index _output_get) _returnvalue _output_get_2) 0 _index) _output_get_2))

(fn `GetCaseLocation`
  (params (Index :type Integer))
  (returns (Location :type "Vector Structure"))
  (return (`self.K2_GetActorLocation` (`|GetArrayItem` (`self.Case`) Index))))

(fn `GetlastIndex`
  (returns (Index :type Integer))
  (return (- (`KismetArrayLibrary.Array_Length` (`self.Case`)) 1)))

(fn `UserConstructionScript`)