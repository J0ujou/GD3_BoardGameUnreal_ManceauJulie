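; Player pawn for a dice board game that walks space by space along a Board of cases.
; BeginPlay restores the active player's saved position from BP_GameInstance; Space rolls the Dice, whose result drives Move, and A forces a six-step debug move.
; Recursive MoveOneStep interpolates the capsule between cases, reversing at the last one on overshoot.
; On arrival it saves the position, then prints a win or triggers the landed case.
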(event `Key|A`
  (params (Key :type "Key Structure"))
  (:`Pressed`
    (`self.Move` 6)
    (`KismetSystemLibrary.PrintString` "kk")))

(event `Key|SpaceBar`
  (params (Key :type "Key Structure"))
  (:`Pressed`
    (if (not (`self.IsMoving`))
      (`KismetSystemLibrary.PrintString` "Hello")
      (`/Game/Blueprints/BP_Dice.RollDice` (`self.Dice`) 0))))

(event `self.ReceiveBeginPlay`
  (bind _gi (`self.GI`))
  ; remet à jour/ à 0...
  (bind _asbp_game_instance (cast `/Game/Blueprints/BP_GameInstance` (`GameplayStatics.GetGameInstance`)))
  (bind _output_get (set `self.GI` _asbp_game_instance))
  (`/Game/Blueprints/BP_GameInstance.EnsureSize` _output_get 1)
  (bind _output_get_2 (set `self.ActualPosition` (`|GetArrayItem` (`/Game/Blueprints/BP_GameInstance.PositionPlayer` _gi) (`/Game/Blueprints/BP_GameInstance.ActualPlayer` _gi))))
  (bind _loc (`self.GetGoal` _output_get_2))
  (`self.K2_SetActorLocation` _loc)
  (add `/Game/Blueprints/BP_Dice.RollDice` (`self.Dice`) (delegate `handleDiceRolled`)))

(event `handleDiceRolled`
  (params (result :type Integer))
  (`self.Move` result))

(event `Move`
  (params (Number :type Integer))
  (if (not (`self.IsMoving`))
    (set `self.IsMoving` true)
    (bind (_newposition _rebound) (`/Game/Blueprints/BP_Board.CalculateNewPosition` (`self.Board`) (`self.ActualPosition`) Number))
    (set `self.EndPosition` _newposition)
    (set `self.Rebound` _rebound)
    (set `self.GoingBack` (< Number 0))
    (`self.MoveOneStep`)))

(event `MoveOneStep`
  (`KismetSystemLibrary.PrintString` (`KismetStringLibrary.Conv_BoolToString` (`self.Rebound`)))
  (if (or (!= (`self.ActualPosition`) (`self.EndPosition`)) (and (`self.Rebound`) (not (`self.GoingBack`))))
    (bind _index (`/Game/Blueprints/BP_Board.GetlastIndex` (`self.Board`)))
    (if (and (`self.Rebound`) (== (`self.ActualPosition`) _index))
      (bind _output_get (set `self.GoingBack` true)))
    (bind _output_get_2 (set `self.NextIndex` (+ (`self.ActualPosition`) (`KismetMathLibrary.SelectInt` -1 1 _output_get))))
    (bind _loc (`self.GetGoal` _output_get_2))
    (`KismetSystemLibrary.MoveComponentTo` (`self.CapsuleComponent`) _loc (struct) false false 0.3)
    (set `self.ActualPosition` (`self.NextIndex`))
    (`self.MoveOneStep`)
    (else
      (set `self.IsMoving` false)
      (`self.SavePosition`)
      (bind _index_2 (`/Game/Blueprints/BP_Board.GetlastIndex` (`self.Board`)))
      (if (== _index_2 (`self.ActualPosition`))
        (`KismetSystemLibrary.PrintString` "win")
        (set `self.IsMoving` true)
        (else
          (`/Game/Blueprints/BP_Case.Trigger` (`|GetArrayItem` (`/Game/Blueprints/BP_Board.Case` (`self.Board`)) (`self.ActualPosition`)) self))))))

(fn `GetGoal`
  (params (Index :type Integer))
  (returns (Loc :type "Vector Structure"))
  (bind _location (`/Game/Blueprints/BP_Board.GetCaseLocation` (`self.Board`) Index))
  (return (`KismetMathLibrary.MakeVector` (.x _location) (.y _location) (`self.PlayerHeight`))))

(fn `SavePosition`
  (bind _gi (`self.GI`))
  (`KismetArrayLibrary.Array_Set` (`/Game/Blueprints/BP_GameInstance.PositionPlayer` _gi) (`/Game/Blueprints/BP_GameInstance.ActualPlayer` _gi) (`self.ActualPosition`)))

(fn `UserConstructionScript`)